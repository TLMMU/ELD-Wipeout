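; BP_SpawnObjectOnTrack is a placeable spawner that populates the stretch of track inside its sphere with actors of a configurable class.
; On BeginPlay it sizes the sphere, finds the BP_TrackSpline actor and samples its spline at evenly spaced distances set by NumberOfPoints.
; Each sample within the sphere radius gets an actor spawned at the spline's location and rotation.
; A tangent-angle range check is left unconnected and never runs.
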(event `self.ReceiveBeginPlay`
  (`SphereComponent.SetSphereRadius` (`self.Sphere`) (`self.Sphere Radius`) true)
  (bind _returnvalue (`GameplayStatics.GetActorOfClass` "/Game/Blueprints/BP_TrackSpline.BP_TrackSpline_C"))
  (for _index (range (+ (`self.Number of Points`) 1))
    (bind _spline (`/Game/Blueprints/BP_TrackSpline.Spline` _returnvalue))
    (bind _returnvalue_2 (* _index (/ (`SplineComponent.GetSplineLength` _spline) (`self.Number of Points`))))
    (bind _returnvalue_3 (`SplineComponent.GetLocationAtDistanceAlongSpline` _spline _returnvalue_2 "World"))
    (if (<= (`KismetMathLibrary.VSize` (- (`SceneComponent.K2_GetComponentLocation` (`self.Sphere`)) _returnvalue_3)) (`self.Sphere Radius`))
      (`|SpawnActorFromClass` (`self.Class`) (`KismetMathLibrary.MakeTransform` _returnvalue_3 (`SplineComponent.GetRotationAtDistanceAlongSpline` _spline _returnvalue_2 "World")) "Undefined" "MultiplyWithRoot" null null))))

(fn `UserConstructionScript`)