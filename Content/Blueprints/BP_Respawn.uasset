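; BP_Respawn is a trigger box actor that sends the player back to a checkpoint when they touch it.
; On BeginPlay it caches every BP_Checkpoint in the level into an array.
; When an actor tagged Player begins overlapping the box, it finds the checkpoint nearest to that actor and teleports the actor to that checkpoint's location and rotation.
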(event `self.ReceiveBeginPlay`
  ; Gets all the checkpoints in the level and adds them to an array.
  (bind _outactors (`GameplayStatics.GetAllActorsOfClass` "/Game/Blueprints/BP_Checkpoint.BP_Checkpoint_C"))
  (set `self.Checkpoints` _outactors))

(event `self.Box.OnComponentBeginOverlap`
  (params (OverlappedComponent :type "PrimitiveComponent Object Reference") (OtherActor :type "Actor Object Reference") (OtherComp :type "PrimitiveComponent Object Reference") (OtherBodyIndex :type Integer) (bFromSweep :type Boolean) (SweepResult :type "HitResult Structure (by ref)"))
  (bind (_distance _returnvalue) (`GameplayStatics.FindNearestActor` (`self.K2_GetActorLocation` OtherActor) (`self.Checkpoints`)))
  ; When the player collides, it will teleport the player to the nearest checkpoint.
  (if (`self.ActorHasTag` OtherActor "Player")
    (`self.K2_SetActorLocationAndRotation` OtherActor (`self.K2_GetActorLocation` _returnvalue) (`self.K2_GetActorRotation` _returnvalue) false false)))

(fn `UserConstructionScript`)