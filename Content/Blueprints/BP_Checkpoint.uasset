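; Checkpoint actor that flashes green when a Player-tagged actor enters its box trigger.
; On BeginPlay it creates one dynamic material for both wall lamps and another for both warning-line meshes, so each pair changes colour together.
; On overlap it recolours those materials, two rect lights and a text render, then a two-second timer restores the default colour.
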(event `self.ReceiveBeginPlay`
  ; Creates 2 arrays for the 2 types of meshes and sets the correct material to them.
  (`|ExecutionSequence`
    (:`then_0`
      (set `self.LampMeshArray` (`|MakeArray` (`self.SM_Wall_lamp_Left`) (`self.SM_Wall_lamp_Right`)))
      (bind _returnvalue (`PrimitiveComponent.CreateDynamicMaterialInstance` (`self.SM_Wall_lamp_Left`) 1 "/Game/Materials/M_EmissiveCheckpoint.M_EmissiveCheckpoint" "None"))
      (set `self.LampMaterial` _returnvalue)
      (for _array_element (`self.LampMeshArray`)
        (`PrimitiveComponent.SetMaterial` _array_element 1 (`self.LampMaterial`))))
    (:`then_1`
      (set `self.WarningLinesMeshArray` (`|MakeArray` (`self.SM_CheckpointWarningLines_Left`) (`self.SM_CheckpointWarningLines_Right`)))
      (bind _returnvalue_2 (`PrimitiveComponent.CreateDynamicMaterialInstance` (`self.SM_CheckpointWarningLines_Left`) 0 "/Game/Materials/M_CheckpointLines.M_CheckpointLines" "None"))
      (set `self.WarningLinesMat` _returnvalue_2)
      (for _array_element_2 (`self.WarningLinesMeshArray`)
        (`PrimitiveComponent.SetMaterial` _array_element_2 0 (`self.WarningLinesMat`))))))

(event `self.Box.OnComponentBeginOverlap`
  (params (OverlappedComponent :type "PrimitiveComponent Object Reference") (OtherActor :type "Actor Object Reference") (OtherComp :type "PrimitiveComponent Object Reference") (OtherBodyIndex :type Integer) (bFromSweep :type Boolean) (SweepResult :type "HitResult Structure (by ref)"))
  (bind _greencolour (`self.GreenColour`))
  (bind _greencolour_2 (`self.GreenColour`))
  ; Every time the vehicle overlaps, it changes the material colour to green then after two seconds it sets back to its original colour.
  (if (`self.ActorHasTag` OtherActor "Player")
    (`KismetSystemLibrary.K2_SetTimerDelegate` (delegate `BackToDefaultColour`) 2.0)
    (`LightComponent.SetLightColor` (`self.RectLight_Left`) _greencolour true)
    (`LightComponent.SetLightColor` (`self.RectLight_Right`) _greencolour true)
    (`MaterialInstanceDynamic.SetVectorParameterValue` (`self.LampMaterial`) "Colour" _greencolour_2)
    (`MaterialInstanceDynamic.SetVectorParameterValue` (`self.WarningLinesMat`) "Colour" _greencolour_2)
    (`TextRenderComponent.SetTextRenderColor` (`self.TextRender`) (`KismetMathLibrary.Conv_LinearColorToColor` (`self.GreenColour`)))))

(event `BackToDefaultColour`
  (bind _defaultcolour (`self.DefaultColour`))
  (bind _defaultcolour_2 (`self.DefaultColour`))
  ; Every time the vehicle overlaps, it changes the material colour to green then after two seconds it sets back to its original colour.
  (`LightComponent.SetLightColor` (`self.RectLight_Left`) _defaultcolour true)
  (`LightComponent.SetLightColor` (`self.RectLight_Right`) _defaultcolour true)
  (`MaterialInstanceDynamic.SetVectorParameterValue` (`self.LampMaterial`) "Colour" _defaultcolour_2)
  (`MaterialInstanceDynamic.SetVectorParameterValue` (`self.WarningLinesMat`) "Colour" _defaultcolour_2)
  (`TextRenderComponent.SetTextRenderColor` (`self.TextRender`) (`KismetMathLibrary.Conv_LinearColorToColor` (`self.DefaultColour`))))

(fn `UserConstructionScript`)