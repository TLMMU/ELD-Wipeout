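; Hover scene component that acts as a raycast suspension spring, pushing its owner's physics-simulated root body away from surfaces below it.
; BeginPlay caches the root primitive, leaving the component inactive if it is not simulating physics.
; Each tick it traces along its down vector, converting compression and its rate of change into a stiffness-plus-damping force.
; That force is applied along its up vector at the component's location, so off-center placement also produces torque.
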(event `self.ReceiveBeginPlay`
  (bind _asprimitive_component (cast `PrimitiveComponent` (`Actor.RootComponent` (`self.GetOwner`))))
  (bind _output_get (set `self.Ref to Body` _asprimitive_component))
  (if (not (`self.IsSimulatingPhysics` _output_get "None"))
    (set `self.Ref to Body` null)))

(event `self.ReceiveTick`
  (params (DeltaSeconds :type "Float (single-precision)"))
  (bind _returnvalue (`self.K2_GetComponentLocation`))
  (bind _hoverdistance (`self.HoverDistance`))
  (`self.Ref to Body`
    (:`then`
      (bind (_outhit _returnvalue_2) (`KismetSystemLibrary.LineTraceSingle` _returnvalue (- _returnvalue (* (`self.GetUpVector`) (`self.HoverDistance`))) "TraceTypeQuery1" false (`|MakeArray` (`self.GetOwner`)) (select `bool` (`self.Ray`) :`true` "ForOneFrame" :!type "EDrawDebugTrace Enum")))
      (if _returnvalue_2
        (bind _returnvalue_3 (/ (- _hoverdistance (`.Distance` (`GameplayStatics.BreakHitResult` _outhit))) _hoverdistance))
        (set `self.HoverForce` (+ (* (/ (- _returnvalue_3 (`self.PrevCompression`)) (`GameplayStatics.GetWorldDeltaSeconds`)) (`self.Damping`)) (* _returnvalue_3 (`self.Stiffness`))))
        (set `self.PrevCompression` _returnvalue_3)
        (`PrimitiveComponent.AddForceAtLocation` (`self.Ref to Body`) (* (`self.GetUpVector`) (`self.HoverForce`)) (`self.K2_GetComponentLocation`) "None")))
    (:`else`)))