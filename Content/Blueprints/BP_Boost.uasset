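; BP_Boost is a boost pickup or pad that speeds up the hover vehicle and shows an XP popup in the time trial UI.
; On BeginPlay it caches the first UI_TimeTrial widget and BP_HoverVehicle found in the world.
; Any Box overlap boosts that cached vehicle briefly, without checking the overlapping actor, and restarts a Timeline animating the widget's XP text before calling UpdateXPAnim.
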(event `self.ReceiveBeginPlay`
  (bind _foundwidgets (`WidgetBlueprintLibrary.GetAllWidgetsOfClass` "/Game/Blueprints/UI_TimeTrial.UI_TimeTrial_C"))
  (set `self.WidgetRef` (`|GetArrayItem` _foundwidgets))
  (bind _outactors (`GameplayStatics.GetAllActorsOfClass` "/Game/Blueprints/BP_HoverVehicle.BP_HoverVehicle_C"))
  (set `self.HoverVehicleRef` (`|GetArrayItem` _outactors)))

(event `self.Box.OnComponentBeginOverlap`
  (params (OverlappedComponent :type "PrimitiveComponent Object Reference") (OtherActor :type "Actor Object Reference") (OtherComp :type "PrimitiveComponent Object Reference") (OtherBodyIndex :type Integer) (bFromSweep :type Boolean) (SweepResult :type "HitResult Structure (by ref)"))
  (`/Game/Blueprints/BP_HoverVehicle.Boost` (`self.HoverVehicleRef`) 1.8 1.0)
  (bind (_direction _textscale _textfloatup) (`Timeline|Timeline` :!via `PlayFromStart`)
    (:`Update`
      (`/Game/Blueprints/UI_TimeTrial.SetXP` (`self.WidgetRef`) _textscale)
      (`/Game/Blueprints/UI_TimeTrial.XPAddAnim` (`self.WidgetRef`) _textfloatup))
    (:`Finished`
      (`/Game/Blueprints/UI_TimeTrial.UpdateXP&Anim` (`self.WidgetRef`)))))

(fn `UserConstructionScript`)