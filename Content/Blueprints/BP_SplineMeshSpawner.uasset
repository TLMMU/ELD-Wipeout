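; Spline mesh spawner Blueprint, apparently unfinished, with math for orienting mesh segments by parallel transport along a curve.
; ParallelTransport rotates a vector by the angle between two tangents around their cross product.
; AddTransportedMesh uses it to derive an up vector and end-point roll difference, but reads a zero transported normal and never applies the result.
; MakeSplineMesh and the event graph are empty, so nothing spawns.
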(fn `AddTransportedMesh`
  (params (`Transport Vector` :type "Vector Structure") (`Start Tangent` :type "Vector Structure") (`End Tangent` :type "Vector Structure"))
  (`self.ParallelTransport` (`KismetMathLibrary.Normal` `Start Tangent`) (`KismetMathLibrary.Normal` `End Tangent`) `Transport Vector`)
  (set `self.Transported Normal Vector` (0.0 0.0 0.0))
  (set `self.UpVector` (/ (+ (`self.Transport Vector`) (`self.Transported Normal Vector`)) 2.0))
  (set `self.Start Point Spline Mesh Right Vector` (`KismetMathLibrary.Normal` (`KismetMathLibrary.Cross_VectorVector` (`self.Start Tangent`) (`self.UpVector`))))
  (set `self.End Point Spline Mesh Right Vector` (`KismetMathLibrary.Normal` (`KismetMathLibrary.Cross_VectorVector` (`self.End Tangent`) (`self.UpVector`))))
  (set `self.End Point Right Vector` (`KismetMathLibrary.Normal` (`KismetMathLibrary.Cross_VectorVector` (`self.End Tangent`) (`self.Transported Normal Vector`))))
  (set `self.Angle Difference` (`KismetMathLibrary.DegAcos` (`KismetMathLibrary.Dot_VectorVector` (`self.End Point Right Vector`) (`self.End Point Spline Mesh Right Vector`)))))

(fn `MakeSplineMesh`
  (params (NewParam :type "Vector Structure")))

(fn `ParallelTransport`
  (params (`Tangent 1` :type "Vector Structure") (`Tangent 2` :type "Vector Structure") (`Transport Vector` :type "Vector Structure"))
  (returns (`Return Value` :type "Vector Structure"))
  (set `self.TangentCross` (`KismetMathLibrary.Cross_VectorVector` `Tangent 1` `Tangent 2`))
  (if (`KismetMathLibrary.Vector_IsZero` (`self.TangentCross`))
    (return (`self.Transport Vector`))
    (else
      (set `self.TangentCross` (`KismetMathLibrary.Normal` (`self.TangentCross`)))
      (return (`KismetMathLibrary.RotateAngleAxis` (`self.Transport Vector`) (`KismetMathLibrary.DegAcos` (`KismetMathLibrary.Dot_VectorVector` (`self.Tangent 1`) (`self.Tangent 2`))) (`self.TangentCross`))))))