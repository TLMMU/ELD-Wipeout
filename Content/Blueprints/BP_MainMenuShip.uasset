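; BP_MainMenuShip is the main menu's spaceship, which hovers in place and does a barrel roll when the player presses Enter.
; Tick fakes the hover by adding small sine-of-time deltas to the Spaceship component's height, roll and yaw.
; StartShipRotation, gated by a DoOnce, plays a timeline whose RotationAlpha output directly sets the Arrow component's world roll while preserving its pitch and yaw.
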(event `self.ReceiveTick`
  (params (DeltaSeconds :type "Float (single-precision)"))
  (bind _returnvalue (`KismetMathLibrary.Sin` (`self.GetGameTimeSinceCreation`)))
  (bind _returnvalue_2 (* _returnvalue 0.1))
  ; Fakes the ship's hovering.
  (`SceneComponent.K2_AddRelativeLocation` (`self.spaceship`) (`KismetMathLibrary.MakeVector` 0.0 0.0 (* _returnvalue 0.1)) false false)
  (`SceneComponent.K2_AddRelativeRotation` (`self.spaceship`) (`KismetMathLibrary.MakeRotator` _returnvalue_2 0.0 _returnvalue_2) false false))

(event `StartShipRotation`
  (bind (_returnvalue_roll _returnvalue_pitch _returnvalue_yaw) (`KismetMathLibrary.BreakRotator` (`SceneComponent.K2_GetComponentRotation` (`self.Arrow`))))
  ; This makes the ship do a barrel roll when the player hits the enter key.
  (`/Engine/EditorBlueprintResources/StandardMacros.DoOnce` false
    (:`Completed`
      (bind (_direction _rotationalpha) (`Timeline|Timeline` :`NewTime` _returnvalue_roll :!via `PlayFromStart`)
        (:`Update`
          (`SceneComponent.K2_SetWorldRotation` (`self.Arrow`) (`KismetMathLibrary.MakeRotator` _rotationalpha _returnvalue_pitch _returnvalue_yaw) false false))))))

(fn `UserConstructionScript`)