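; Split turn sign actor that runs an endless chasing light sequence across its front, middle and back meshes.
; On BeginPlay it gives each mesh a dynamic instance of the turn sign light material and stores them in an array.
; A self-restarting timer loop turns one instance's Colour white for half a second, sets it red, then advances the index, wrapping at the end.
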(event `self.ReceiveBeginPlay`
  (bind _turnsignmaterialarray (`self.TurnSignMaterialArray`))
  ; This loops through the mesh array and applies a instance of a material.
  (set `self.MeshArray` (`|MakeArray` (`self.SplitTurnSign_Front`) (`self.SplitTurnSign_Mid`) (`self.SplitTurnSign_Back`)))
  (for _array_element (`self.MeshArray`)
    (bind _returnvalue (`PrimitiveComponent.CreateDynamicMaterialInstance` _array_element 0 "/Game/Materials/M_TurnSignLight.M_TurnSignLight" "None"))
    (bind _returnvalue_2 (`KismetArrayLibrary.Array_Add` _turnsignmaterialarray _returnvalue))
    (`PrimitiveComponent.SetMaterial` (`|GetArrayItem` (`self.MeshArray`) _returnvalue_2) 0 (`|GetArrayItem` _turnsignmaterialarray _returnvalue_2)))
  (`self.StartLightSequenceLoop`))

(event `StartLightSequenceLoop`
  ; This sequentially changes the colour of each turn sign actor in the array then after 0.5 seconds, it sets the colour back to its original. When the index hits is equal to the max length, it sets the index back to zero and starts the event creating an infinite loop.
  (if (== (`self.Index`) (`KismetArrayLibrary.Array_Length` (`self.TurnSignMaterialArray`)))
    (set `self.Index` 0)
    (`self.StartLightSequenceLoop`)
    (else
      (`KismetSystemLibrary.K2_SetTimerDelegate` (delegate `BackToRed`) 0.5)
      (`MaterialInstanceDynamic.SetVectorParameterValue` (`|GetArrayItem` (`self.TurnSignMaterialArray`) (`self.Index`)) "Colour" (struct :`R` 1.0 :`G` 1.0 :`B` 1.0 :`A` 1.0)))))

(event `BackToRed`
  ; This sequentially changes the colour of each turn sign actor in the array then after 0.5 seconds, it sets the colour back to its original. When the index hits is equal to the max length, it sets the index back to zero and starts the event creating an infinite loop.
  (`MaterialInstanceDynamic.SetVectorParameterValue` (`|GetArrayItem` (`self.TurnSignMaterialArray`) (`self.Index`)) "Colour" (struct :`R` 1.0 :`A` 1.0))
  (set `self.Index` (+ (`self.Index`) 1))
  (`self.StartLightSequenceLoop`))

(fn `UserConstructionScript`)