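; Player-driven hover racer built on a physics sphere that aligns to the surface beneath it.
; Smoothed forward input sets acceleration for per-tick impulse thrust, while steer and drift add speed-scaled yaw torque, with steering flipped upside down.
; A downward trace rotates the sphere toward the surface normal and applies custom gravity along it, enabling world gravity on a miss.
; Mesh banking and camera drift rotation are cosmetic offsets that ease back to neutral.
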(event `EnhancedInput|/Game/Input/IA_Forward`
  (params (ActionValue :type "Float (double-precision)") (ElapsedSeconds :type "Float (double-precision)") (TriggeredSeconds :type "Float (double-precision)") (InputAction :type "InputAction Object Reference" :default "/Game/Input/IA_Forward.IA_Forward"))
  (:`Triggered`
    (set `self.AccelerationInput` (`KismetMathLibrary.FInterpTo` (`self.AccelerationInput`) ActionValue (`GameplayStatics.GetWorldDeltaSeconds`) 0.5))))

(event `EnhancedInput|/Game/Input/IA_Drift`
  (params (ActionValue :type "Float (double-precision)") (ElapsedSeconds :type "Float (double-precision)") (TriggeredSeconds :type "Float (double-precision)") (InputAction :type "InputAction Object Reference" :default "/Game/Input/IA_Drift.IA_Drift"))
  (bind _roll (.roll (`self.Relative Rotation Z (Yaw)`)))
  (bind _pitch (.pitch (`self.Relative Rotation Z (Yaw)`)))
  (bind _yaw (.yaw (`self.Relative Rotation Z (Yaw)`)))
  (:`Triggered`
    (`PrimitiveComponent.AddTorqueInRadians` (`self.Sphere`) (`KismetMathLibrary.MakeVector` 0.0 0.0 (`KismetMathLibrary.FInterpTo` ActionValue (* ActionValue 345.0 (`self.AccelerationInput`)) (`GameplayStatics.GetWorldDeltaSeconds`) 3.0)) "None" true)
    (set `self.Relative Rotation Z (Yaw)` (`KismetMathLibrary.RLerp` (`KismetMathLibrary.MakeRotator` _roll _pitch (+ _yaw 0.5)) (`KismetMathLibrary.MakeRotator` _roll _pitch (- _yaw 0.5)) (/ (+ ActionValue 1.0) 2.0)))
    (`KismetSystemLibrary.PrintString` (`KismetStringLibrary.Conv_DoubleToString` ActionValue))))

(event `EnhancedInput|/Game/Input/IA_Steer`
  (params (ActionValue :type "Float (double-precision)") (ElapsedSeconds :type "Float (double-precision)") (TriggeredSeconds :type "Float (double-precision)") (InputAction :type "InputAction Object Reference" :default "/Game/Input/IA_Steer.IA_Steer"))
  (bind _returnvalue (* ActionValue -1.0))
  (bind _originalrollrot (`self.OriginalRollRot`))
  (bind (_returnvalue_x _returnvalue_y _returnvalue_z) (`KismetMathLibrary.BreakVector` (`SceneComponent.GetUpVector` (`self.Sphere`))))
  (bind _returnvalue_2 (/ (+ ActionValue 1.0) 2.0))
  (bind _returnvalue_3 (+ (`self.OriginalPitchRot`) 0.5))
  (:`Triggered`
    (if (`KismetMathLibrary.InRange_FloatFloat` _returnvalue_z -1.0 -0.1 false false)
      (`PrimitiveComponent.AddTorqueInRadians` (`self.Sphere`) (`KismetMathLibrary.MakeVector` 0.0 0.0 (`KismetMathLibrary.FInterpTo` _returnvalue (* _returnvalue 145.0 (`self.AccelerationInput`)) (`GameplayStatics.GetWorldDeltaSeconds`) 3.0)) "None" true)
      (else
        (`PrimitiveComponent.AddTorqueInRadians` (`self.Sphere`) (`KismetMathLibrary.MakeVector` 0.0 0.0 (`KismetMathLibrary.FInterpTo` ActionValue (* ActionValue 145.0 (`self.AccelerationInput`)) (`GameplayStatics.GetWorldDeltaSeconds`) 3.0)) "None" true)))
    (set `self.OriginalRollRot` (`KismetMathLibrary.Lerp` (- _originalrollrot 1.2) (+ _originalrollrot 1.2) _returnvalue_2))
    (set `self.OriginalPitchRot` (`KismetMathLibrary.Lerp` _returnvalue_3 _returnvalue_3 _returnvalue_2))))

(event `self.ReceiveTick`
  (params (DeltaSeconds :type "Float (single-precision)"))
  (bind _sphere (`self.Sphere`))
  (bind _returnvalue (`SceneComponent.K2_GetComponentLocation` _sphere))
  (`self.CalcAcceleration`)
  (`self.Thrust`)
  (bind _output_get (set `self.Relative Rotation Z (Yaw)` (`KismetMathLibrary.RInterpTo` (`self.Relative Rotation Z (Yaw)`) (struct) (`GameplayStatics.GetWorldDeltaSeconds`) 1.0)))
  (`SceneComponent.K2_SetRelativeRotation` (`self.CameraSphere`) _output_get false false)
  (bind (_roll _pitch) (`self.VehicleBanking`))
  (`SceneComponent.K2_SetRelativeRotation` (`self.SM_Racer`) (`KismetMathLibrary.MakeRotator` _roll _pitch) false false)
  ; Aligns the sphere based on surface hit by line trace
  (bind (_outhit _returnvalue_2) (`KismetSystemLibrary.LineTraceSingle` _returnvalue (- _returnvalue (* (`SceneComponent.GetUpVector` _sphere) 170.0)) "TraceTypeQuery1" false (`|MakeArray` (`ActorComponent.GetOwner` (`self.Sphere`)))))
  (if _returnvalue_2
    (bind (_bblockinghit _binitialoverlap _time _distance _location _impactpoint _normal _impactnormal) (`GameplayStatics.BreakHitResult` _outhit))
    (bind _returnvalue_3 (`KismetMathLibrary.Cross_VectorVector` (`SceneComponent.GetUpVector` (`self.Sphere`)) _normal))
    (`SceneComponent.K2_AddWorldRotation` (`self.Sphere`) (`KismetMathLibrary.RotatorFromAxisAndAngle` (`KismetMathLibrary.Normal` _returnvalue_3) (* (`KismetMathLibrary.VSize` _returnvalue_3) 10.0)) false false)
    ; Dynamic gravity that changes based on surface hit by the line trace
    (`PrimitiveComponent.AddForce` (`self.Sphere`) (* (`KismetMathLibrary.Normal` _impactnormal) (`self.GravStrength`)) "None" true)
    (else
      (`SceneComponent.K2_AddWorldRotation` :`self` (`self.Sphere`))
      (`PrimitiveComponent.SetEnableGravity` (`self.Sphere`) true))))

(fn `CalcAcceleration`
  (bind _accelerationinput (`self.AccelerationInput`))
  (set `self.Acceleration` (* (`KismetMathLibrary.Lerp` 0.0 15000.0 _accelerationinput) (/ (+ _accelerationinput 1.0) 2.0)))
  (set `self.AccelerationInput` (`KismetMathLibrary.FInterpTo` (`self.AccelerationInput`) 0.0 (`GameplayStatics.GetWorldDeltaSeconds`) 0.3)))

(fn `Thrust`
  (bind _sphere (`self.Sphere`))
  (`PrimitiveComponent.AddImpulse` (`self.Sphere`) (/ (* (`SceneComponent.GetForwardVector` _sphere) (* (`PrimitiveComponent.GetMass` _sphere) (- (`self.Acceleration`) 0.0))) 200.0) "None" false))

(fn `UserConstructionScript`)

(fn `VehicleBanking`
  (returns (Roll :type "Float (double-precision)") (Pitch :type "Float (double-precision)"))
  (bind _output_get (set `self.OriginalRollRot` (`KismetMathLibrary.FInterpTo` (`self.OriginalRollRot`) 0.0 (`GameplayStatics.GetWorldDeltaSeconds`) 4.0)))
  (bind _output_get_2 (set `self.OriginalPitchRot` (`KismetMathLibrary.FInterpTo` (`self.OriginalPitchRot`) 0.0 (`GameplayStatics.GetWorldDeltaSeconds`) 4.0)))
  (return _output_get _output_get_2))