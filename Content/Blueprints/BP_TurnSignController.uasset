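; Controller that makes nearby BP_TurnSign actors switch colours in sequence.
; On BeginPlay it resizes and nudges its sphere or box to make overlap detection reliable, then collects overlapping signs.
; It swap-sorts them by distance from an Arrow component that marks the sequence start.
; A looping timer, set when a swap occurs, calls StartLoop on one sign per tick, wrapping at the end.
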(event `self.ReceiveBeginPlay`
  (bind _box (`self.Box`))
  (bind _sphere (`self.Sphere`))
  (bind _returnvalue (`SceneComponent.K2_GetComponentLocation` (`self.Arrow`)))
  ; The behaviour of Get Overlapping Actors is unpredictable leading to the controller sometimes failing to detect any actors. I fixed this by the setting the sphere radius/box extent and moving them by a small amount. The overlapping turn signs are added to an array. The arrow's position is moved in the world to the first actor for sorting the array. It is sorted based on the distance between the arrow and actors and it ensures that they are going in order when playing the colour switch loop. A looping timer executes a custom event in one actor after another from the sorted array to continously switch between colours.
  (if (`self.SphereOverlap`)
    (`SphereComponent.SetSphereRadius` (`self.Sphere`) (`self.Sphere Radius`) true)
    (`SceneComponent.K2_SetWorldLocation` _sphere (+ (`SceneComponent.K2_GetComponentLocation` _sphere) (1.0 0.0 0.0)) true false)
    (else
      (`BoxComponent.SetBoxExtent` (`self.Box`) (`self.BoxExtent`) true)
      (`SceneComponent.K2_SetWorldLocation` _box (+ (`SceneComponent.K2_GetComponentLocation` _box) (1.0 0.0 0.0)) true false)))
  (bind _output_get (set `self.TurnSignActorArray` (`self.GetOverlappingActors` "/Game/Blueprints/BP_TurnSign.BP_TurnSign_C")))
  (for (_array_element _array_index) _output_get
    (for _index (range _array_index (`KismetArrayLibrary.Array_Length` _output_get))
      (if (< (`KismetMathLibrary.Vector_Distance` (`self.K2_GetActorLocation` (`|GetArrayItem` _output_get _index)) _returnvalue) (`KismetMathLibrary.Vector_Distance` (`self.K2_GetActorLocation` _array_element) _returnvalue))
        (`KismetArrayLibrary.Array_Swap` (`self.TurnSignActorArray`) _index _array_index)
        (set `self.Index` 0)
        (`KismetSystemLibrary.K2_SetTimerDelegate` (delegate `TurnSignSequenceLoop`) 0.2 true)))))

(event `TurnSignSequenceLoop`
  (bind _turnsignactorarray (`self.TurnSignActorArray`))
  ; The behaviour of Get Overlapping Actors is unpredictable leading to the controller sometimes failing to detect any actors. I fixed this by the setting the sphere radius/box extent and moving them by a small amount. The overlapping turn signs are added to an array. The arrow's position is moved in the world to the first actor for sorting the array. It is sorted based on the distance between the arrow and actors and it ensures that they are going in order when playing the colour switch loop. A looping timer executes a custom event in one actor after another from the sorted array to continously switch between colours.
  (if (< (`self.Index`) (`KismetArrayLibrary.Array_Length` _turnsignactorarray))
    (`/Game/Blueprints/BP_TurnSign.StartLoop` (`|GetArrayItem` _turnsignactorarray (`self.Index`)))
    (set `self.Index` (+ (`self.Index`) 1))
    (else
      (set `self.Index` 0))))

(fn `UserConstructionScript`
  (if (`self.SphereOverlap`)
    (`SphereComponent.SetSphereRadius` (`self.Sphere`) (`self.Sphere Radius`) true)
    (else
      (`BoxComponent.SetBoxExtent` (`self.Box`) (`self.BoxExtent`) true))))