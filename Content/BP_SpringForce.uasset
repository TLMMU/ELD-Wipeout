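; BP_SpringForce is a raycast suspension spring that pushes its owner's static mesh along the surface normal.
; On BeginPlay, when ForceMod is non-zero, it traces down its local up axis over SpringLength.
; On a hit, CalcSpringForce combines compression times stiffness with compression rate times damping, scaled by ForceMod, and applies it at the spring's location.
; The force runs once at BeginPlay, with no per-frame update.
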(event `self.ReceiveBeginPlay`
  (bind _defaultsceneroot (`self.DefaultSceneRoot`))
  (if (!= (`self.ForceMod`) 0.0)
    (set `self.SpringLocation` (`SceneComponent.K2_GetComponentLocation` _defaultsceneroot))
    (bind (_outhit _returnvalue) (`KismetSystemLibrary.LineTraceSingle` (`self.SpringLocation`) (- (`self.SpringLocation`) (* (`SceneComponent.GetUpVector` _defaultsceneroot) (`self.SpringLength`))) "TraceTypeQuery1"))
    (if _returnvalue
      (bind (_bblockinghit _binitialoverlap _time _distance _location _impactpoint _normal) (`GameplayStatics.BreakHitResult` _outhit))
      (bind _force (`self.CalcSpringForce` _distance _normal))
      (`PrimitiveComponent.AddForceAtLocation` (`self.GetComponentByClass` (`self.GetOwner`) "/Script/Engine.StaticMeshComponent") _force (`SceneComponent.K2_GetComponentLocation` (`self.DefaultSceneRoot`)) "None")
      (set `self.SuspensionPrev` (`self.SuspensionDelta`)))))

(fn `CalcSpringForce`
  (params (Distance :type "Float (double-precision)") (Normal :type "Vector Structure"))
  (returns (Force :type "Vector Structure"))
  (set `self.SuspensionDelta` (- (`self.SpringLength`) Distance))
  (return (* Normal (* (+ (* (`self.SuspensionDelta`) (`self.Stiffness`)) (* (/ (- (`self.SuspensionDelta`) (`self.SuspensionPrev`)) (`GameplayStatics.GetWorldDeltaSeconds`)) (`self.Damping`))) (`self.ForceMod`)))))

(fn `UserConstructionScript`)