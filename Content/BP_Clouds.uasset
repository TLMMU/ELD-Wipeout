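; Cloud actor that fakes a volumetric cloud layer by stacking static mesh slices at runtime.
; On BeginPlay it adds mesh components at Z steps of VolumeHeight divided by VolumeResolution.
; The base Plane and each slice get a dynamic material instance fed the base world height and VolumeHeight as MinFrom and MaxFrom.
; A leftover debug print fires for every slice.
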(event `self.ReceiveBeginPlay`
  (bind _plane (`self.Plane`))
  (bind (_returnvalue_x _returnvalue_y _returnvalue_z) (`KismetMathLibrary.BreakVector` (`SceneComponent.K2_GetComponentLocation` _plane)))
  (bind _returnvalue (+ (`self.PreviousLayerHeight`) (/ (`self.VolumeHeight`) (`self.VolumeResolution`))))
  (bind _returnvalue_2 (`PrimitiveComponent.CreateDynamicMaterialInstance` _plane 0 (`PrimitiveComponent.GetMaterial` (`self.Plane`) 0) "None"))
  (set `self.SeedHeight` _returnvalue_z)
  (`MaterialInstanceDynamic.SetScalarParameterValue` _returnvalue_2 "MinFrom" _returnvalue_z)
  (`MaterialInstanceDynamic.SetScalarParameterValue` _returnvalue_2 "MaxFrom" (`self.VolumeHeight`))
  (for _ (range (+ (`self.VolumeResolution`) 1))
    (bind _returnvalue_3 (`AddComponent|NODE_AddStaticMeshComponent-0` :`RelativeTransform` (`KismetMathLibrary.MakeTransform` (`KismetMathLibrary.MakeVector` 0.0 0.0 _returnvalue))))
    (set `self.PreviousLayerHeight` _returnvalue)
    (bind _returnvalue_4 (`PrimitiveComponent.CreateDynamicMaterialInstance` _returnvalue_3 0 (`PrimitiveComponent.GetMaterial` _returnvalue_3 0) "None"))
    (`MaterialInstanceDynamic.SetScalarParameterValue` _returnvalue_4 "MinFrom" (`self.SeedHeight`))
    (`MaterialInstanceDynamic.SetScalarParameterValue` _returnvalue_4 "MaxFrom" (`self.VolumeHeight`))
    (`KismetSystemLibrary.PrintString` (`KismetStringLibrary.Conv_DoubleToString` 0.0) true true (struct :`G` 0.66 :`B` 1.0 :`A` 1.0) 10.0)))

(fn `UserConstructionScript`)